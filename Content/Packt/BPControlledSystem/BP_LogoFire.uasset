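; BP_LogoFire is an actor that displays a logo on a plane together with a Niagara fire effect driven by the same texture.
; Its construction script passes FireDensity, FireColor and Texture to Niagara user parameters.
; It also creates a dynamic instance of M_packtlogo_Mat on the plane, sharing that texture and color so logo and fire match.
; The event graph holds no active logic.
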(event EventBeginPlay)

(event Collision|EventActorBeginOverlap
  (params (OtherActor :type Actor%20Object%20Reference)))

(event EventTick
  (params (DeltaSeconds :type Float%20%28single-precision%29)))

(fn ConstructionScript
  (Niagara|SetNiagaraVariable(Float) (Variables|Default|GetNiagaraFire) "User.FireDensity" (Variables|PacktAttributes|GetFireDensity))
  (Niagara|SetTextureObject (Variables|Default|GetNiagaraFire) "User.Texture" (Variables|PacktAttributes|GetTexture))
  (bind _returnvalue (Rendering|Material|CreateDynamicMaterialInstance (Variables|Default|GetPlane) 0 "/Game/Packt/BPControlledSystem/M_packtlogo_Mat.M_packtlogo_Mat" "None" :!class /Script/Engine.PrimitiveComponent))
  (Rendering|Material|SetTextureParameterValue _returnvalue "TextureUsed" (Variables|PacktAttributes|GetTexture))
  (Rendering|Material|SetVectorParameterValue _returnvalue "LogoColor" (Variables|PacktAttributes|GetFireColor) :!class /Script/Engine.MaterialInstanceDynamic)
  (Niagara|SetNiagaraVariable(LinearColor) (Variables|Default|GetNiagaraFire) "User.FireColor" (Variables|PacktAttributes|GetFireColor)))